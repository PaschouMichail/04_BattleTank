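; Mortar actor Blueprint with a barrel, turret and a health bar widget.
; On BeginPlay it initializes its TankAiming component with the mortar barrel and turret.
; It then hands itself to the HealthBarMortar widget so the bar can reference its owning mortar.
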(event `self.ReceiveBeginPlay`
  (`TankAimingComponent.Initialize` (`self.TankAiming`) (`self.Mortar Barrel`) (`self.MortarTurret`))
  (`self.Initialize Health bar`))

(fn `Initialize Health bar`
  (bind _ashealth_bar_mortar (cast `/Game/UI/HealthBarMortar` (`WidgetComponent.GetUserWidgetObject` (`self.Widget`))))
  (set `/Game/UI/HealthBarMortar.MyMortar` self _ashealth_bar_mortar))

(fn `UserConstructionScript`)